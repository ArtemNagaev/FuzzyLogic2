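; GM_Salad, by its name a game mode, provides two functions that classify CL ratio and turbidity readings into enum levels.
; Each samples two curves at the input, fuzzy-membership style, and picks the stronger: Medium versus High for CL ratio, Low versus High for turbidity.
; Near-equal values favor the lower level, and a fallback enum value covers neither matching.
; BeginPlay, Tick and the construction script are empty.
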(event `self.ReceiveBeginPlay`)

(event `self.ReceiveTick`
  (params (DeltaSeconds :type "Float (single-precision)")))

(fn `Check_CL_ratio`
  (params (InputValue :type "Float (double-precision)"))
  (returns (NewParam :type "/Game/Blueprints/LowMediumHigh Enum"))
  (locals (Medium :type "CurveFloat Object Reference" :default "CurveFloat'/Game/Blueprints/Curves/CL_ratio/CL_ratio_Medium.CL_ratio_Medium'") (High :type "CurveFloat Object Reference" :default "CurveFloat'/Game/Blueprints/Curves/CL_ratio/CL_ratio_High.CL_ratio_High'") (InputValueLoc :type "Float (double-precision)"))
  (bind _returnvalue (`CurveFloat.GetFloatValue` (`local.High`) (`local.InputValueLoc`)))
  (bind _returnvalue_2 (`CurveFloat.GetFloatValue` (`local.Medium`) (`local.InputValueLoc`)))
  (bind _returnvalue_3 (`KismetMathLibrary.FMax` _returnvalue_2 _returnvalue))
  (set `local.InputValueLoc` InputValue)
  (if (`KismetMathLibrary.NearlyEqual_FloatFloat` _returnvalue_2 _returnvalue_3)
    (return "NewEnumerator1")
    (elif (`KismetMathLibrary.NearlyEqual_FloatFloat` _returnvalue_3 _returnvalue)
      (return "NewEnumerator2")
      (else
        (return "NewEnumerator3")))))

(fn `Check_Turbidity`
  (params (InputValue :type "Float (double-precision)"))
  (returns (NewParam :type "/Game/Blueprints/LowMediumHigh Enum"))
  (locals (Low :type "CurveFloat Object Reference" :default "CurveFloat'/Game/Blueprints/Curves/Turbidity/Turbidity_Low.Turbidity_Low'") (High :type "CurveFloat Object Reference" :default "CurveFloat'/Game/Blueprints/Curves/Turbidity/Turbidity_High.Turbidity_High'") (InputValueLoc :type "Float (double-precision)"))
  (bind _returnvalue (`CurveFloat.GetFloatValue` (`local.High`) (`local.InputValueLoc`)))
  (bind _returnvalue_2 (`CurveFloat.GetFloatValue` (`local.Low`) (`local.InputValueLoc`)))
  (bind _returnvalue_3 (`KismetMathLibrary.FMax` _returnvalue_2 _returnvalue))
  (set `local.InputValueLoc` InputValue)
  (if (`KismetMathLibrary.NearlyEqual_FloatFloat` _returnvalue_2 _returnvalue_3)
    (return "NewEnumerator0")
    (elif (`KismetMathLibrary.NearlyEqual_FloatFloat` _returnvalue_3 _returnvalue)
      (return "NewEnumerator2")
      (else
        (return "NewEnumerator3")))))

(fn `UserConstructionScript`)