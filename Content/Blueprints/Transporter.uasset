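; Transporter actor that simulates what appears to be water treatment, using fuzzy-style rules to regulate turbidity, microbe and chlorine levels.
; Each tick, Update integrates speed, water flow and chlorine rates into those levels with random drift.
; Rules then classify values by the highest of their membership curves and set the rates for later ticks, which persist until another rule overwrites them.
; Progress logic is disconnected, and LinearMove is never called here.
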(event `self.ReceiveBeginPlay`
  (set `self.Turbidity` (`KismetMathLibrary.RandomFloatInRange` 0.0 80.0)))

(event `self.ReceiveTick`
  (params (DeltaSeconds :type "Float (single-precision)"))
  (`|ExecutionSequence`
    (:`then_0`
      (`self.Update`))
    (:`then_1`
      (bind _linguisticdescription (`self.Check2Function` (`self.Turbidity`) "/Game/Blueprints/Curves/Turbidity/Turbidity_Low.Turbidity_Low" "/Game/Blueprints/Curves/Turbidity/Turbidity_High.Turbidity_High"))
      (bind _linguisticdescription_2 (`self.Check2Function` (`self.WaterFlow`) "/Game/Blueprints/Curves/Water_f/Water_f_low.Water_f_low" "/Game/Blueprints/Curves/Water_f/Water_f_high.Water_f_high"))
      (if (and (`|EnumEquality` _linguisticdescription_2 "NewEnumerator0") (`|EnumEquality` _linguisticdescription "NewEnumerator2"))
        (set `self.WaterFlow_var` 0.5)))
    (:`then_2`
      (bind _linguisticdescription_3 (`self.Check2Function` (`self.Turbidity`) "/Game/Blueprints/Curves/Turbidity/Turbidity_Low.Turbidity_Low" "/Game/Blueprints/Curves/Turbidity/Turbidity_High.Turbidity_High"))
      (bind _linguisticdescription_4 (`self.Check2Function` (`self.WaterFlow`) "/Game/Blueprints/Curves/Water_f/Water_f_low.Water_f_low" "/Game/Blueprints/Curves/Water_f/Water_f_high.Water_f_high"))
      (if (and (`|EnumEquality` _linguisticdescription_4 "NewEnumerator2") (`|EnumEquality` _linguisticdescription_3 "NewEnumerator2"))
        (set `self.Speed_var` -0.5)))
    (:`then_3`
      (bind _linguisticdescription_5 (`self.Check2Function` (`self.Turbidity`) "/Game/Blueprints/Curves/Turbidity/Turbidity_Low.Turbidity_Low" "/Game/Blueprints/Curves/Turbidity/Turbidity_High.Turbidity_High"))
      (bind _linguisticdescription_6 (`self.Check2Function` (`self.Speed_var`) "/Game/Blueprints/Curves/Speed/Speed_low.Speed_low" "/Game/Blueprints/Curves/Speed/Speed_high.Speed_high"))
      (if (and (`|EnumEquality` _linguisticdescription_6 "NewEnumerator0") (`|EnumEquality` _linguisticdescription_5 "NewEnumerator0"))
        (set `self.Speed_var` 0.5)))
    (:`then_4`
      (bind _linguisticdescription_7 (`self.Check2Function` (`self.Turbidity`) "/Game/Blueprints/Curves/Turbidity/Turbidity_Low.Turbidity_Low" "/Game/Blueprints/Curves/Turbidity/Turbidity_High.Turbidity_High"))
      (bind _linguisticdescription_8 (`self.Check2Function` (`self.Speed`) "/Game/Blueprints/Curves/Speed/Speed_low.Speed_low" "/Game/Blueprints/Curves/Speed/Speed_high.Speed_high"))
      (if (and (`|EnumEquality` _linguisticdescription_8 "NewEnumerator2") (`|EnumEquality` _linguisticdescription_7 "NewEnumerator0"))
        (set `self.WaterFlow_var` -0.5)))
    (:`then_5`
      (bind _linguisticdescription_9 (`self.Check3Function` (`self.MicroRatio`) "/Game/Blueprints/Curves/TMicro_ratio/TMicro_ratio_Low.TMicro_ratio_Low" "/Game/Blueprints/Curves/TMicro_ratio/TMicro_ratio_Medium.TMicro_ratio_Medium" "/Game/Blueprints/Curves/TMicro_ratio/TMicro_ratio_high.TMicro_ratio_high"))
      (if (`|EnumEquality` _linguisticdescription_9 "NewEnumerator2")
        (set `self.ChlorineFlow_var` 1.0)))
    (:`then_6`
      (bind _linguisticdescription_10 (`self.Check3Function` (`self.MicroRatio`) "/Game/Blueprints/Curves/TMicro_ratio/TMicro_ratio_Low.TMicro_ratio_Low" "/Game/Blueprints/Curves/TMicro_ratio/TMicro_ratio_Medium.TMicro_ratio_Medium" "/Game/Blueprints/Curves/TMicro_ratio/TMicro_ratio_high.TMicro_ratio_high"))
      (bind _linguisticdescription_11 (`self.Check2Function` (`self.ChlorineRatio`) "/Game/Blueprints/Curves/CL_ratio/CL_ratio_Medium.CL_ratio_Medium" "/Game/Blueprints/Curves/CL_ratio/CL_ratio_High.CL_ratio_High"))
      (if (and (`|EnumEquality` _linguisticdescription_11 "NewEnumerator2") (`|EnumEquality` _linguisticdescription_10 "NewEnumerator0"))
        (set `self.ChlorineFlow_var` -1.0)))))

(fn `Check2Function`
  (params (Value :type "Float (double-precision)") (LowCurve :type "CurveFloat Object Reference") (HighCurve :type "CurveFloat Object Reference"))
  (returns (LinguisticDescription :type "/Game/Blueprints/LowMediumHigh Enum"))
  (locals (ValueLocal :type "Float (double-precision)") (LowLocal :type "CurveFloat Object Reference") (HighLocal :type "CurveFloat Object Reference") (MaxValueLocal :type "Float (double-precision)" :default 0.0))
  (set `local.ValueLocal` Value)
  (set `local.LowLocal` LowCurve)
  (set `local.HighLocal` HighCurve)
  (set `local.MaxValueLocal` (`KismetMathLibrary.FMax` (`CurveFloat.GetFloatValue` (`local.LowLocal`) (`local.ValueLocal`)) 0.0 (`CurveFloat.GetFloatValue` (`local.HighLocal`) (`local.ValueLocal`))))
  (if (== (`local.MaxValueLocal`) (`CurveFloat.GetFloatValue` (`local.LowLocal`) (`local.ValueLocal`)))
    (return "NewEnumerator0")
    (elif (== (`local.MaxValueLocal`) (`CurveFloat.GetFloatValue` (`local.HighLocal`) (`local.ValueLocal`)))
      (return "NewEnumerator2")
      (else
        (return "NewEnumerator3")))))

(fn `Check3Function`
  (params (Value :type "Float (double-precision)") (LowCurve :type "CurveFloat Object Reference") (MediumCurve :type "CurveFloat Object Reference") (HighCurve :type "CurveFloat Object Reference"))
  (returns (LinguisticDescription :type "/Game/Blueprints/LowMediumHigh Enum"))
  (locals (ValueLocal :type "Float (double-precision)") (LowLocal :type "CurveFloat Object Reference") (MediumLocal :type "CurveFloat Object Reference") (HighLocal :type "CurveFloat Object Reference") (MaxValueLocal :type "Float (double-precision)" :default 0.0))
  (set `local.ValueLocal` Value)
  (set `local.LowLocal` LowCurve)
  (set `local.MediumLocal` MediumCurve)
  (set `local.HighLocal` HighCurve)
  (set `local.MaxValueLocal` (`KismetMathLibrary.FMax` (`CurveFloat.GetFloatValue` (`local.LowLocal`) (`local.ValueLocal`)) (`CurveFloat.GetFloatValue` (`local.MediumLocal`) (`local.ValueLocal`)) (`CurveFloat.GetFloatValue` (`local.HighLocal`) (`local.ValueLocal`))))
  (if (== (`local.MaxValueLocal`) (`CurveFloat.GetFloatValue` (`local.LowLocal`) (`local.ValueLocal`)))
    (return "NewEnumerator0")
    (elif (== (`local.MaxValueLocal`) (`CurveFloat.GetFloatValue` (`local.MediumLocal`) (`local.ValueLocal`)))
      (return "NewEnumerator1")
      (elif (== (`local.MaxValueLocal`) (`CurveFloat.GetFloatValue` (`local.HighLocal`) (`local.ValueLocal`)))
        (return "NewEnumerator2")
        (else
          (return "NewEnumerator3"))))))

(fn `LinearMove`
  (params (Start :type "Float (double-precision)") (End :type "Float (double-precision)") (Object :type "Pawn Object Reference"))
  (bind _returnvalue (`SceneComponent.K2_GetComponentToWorld` (`Actor.RootComponent` Object)))
  (`SceneComponent.K2_SetWorldLocation` (`self.RootComponent`) (`KismetMathLibrary.MakeVector` (.x (.location _returnvalue)) (.y (.location _returnvalue))) false false))

(fn `Update`
  (bind _output_get (set `self.ChlorineRatio` (+ (`self.ChlorineRatio`) (`self.ChlorineFlow_var`))))
  (set `self.ChlorineRatio` (`KismetMathLibrary.FMax` _output_get))
  (set `self.MicroRatio` (- (`self.MicroRatio`) (`KismetMathLibrary.FMax` (`self.ChlorineFlow_var`))))
  (bind _output_get_2 (set `self.Speed` (+ (`self.Speed`) (`self.Speed_var`))))
  (set `self.Speed` (`KismetMathLibrary.FMin` _output_get_2 90.0))
  (bind _output_get_3 (set `self.WaterFlow` (+ (`self.WaterFlow`) (`self.WaterFlow_var`))))
  (set `self.WaterFlow` (`KismetMathLibrary.FMin` _output_get_3 90.0))
  (set `self.Turbidity` (+ (- (`self.Turbidity`) (/ (`self.WaterFlow_var`) 2.0)) (/ (`self.Speed_var`) 2.0)))
  (set `self.Turbidity` (+ (`self.Turbidity`) (`KismetMathLibrary.RandomFloatInRange` 0.0 0.1)))
  (set `self.MicroRatio` (+ (`self.MicroRatio`) (`KismetMathLibrary.RandomFloatInRange` 0.0 0.2))))

(fn `UserConstructionScript`)